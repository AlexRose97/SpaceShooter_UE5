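; BP_Bullet is a projectile for the space shooter, serving both player and enemy shots according to its own actor tag.
; Every Tick it moves along its forward vector at Speed, without sweeping.
; On overlap, enemy bullets damage the player's BP_Character, while player bullets apply no damage to enemies here.
; Both hit types spawn an explosion and sound, then destroy the bullet after a short delay; limit-tagged boundaries destroy it silently.
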(event `self.ReceiveTick`
  (params (DeltaSeconds :type "Float (single-precision)"))
  (`self.Move` DeltaSeconds))

(event `self.ReceiveActorBeginOverlap`
  (params (OtherActor :type "Actor Object Reference"))
  (bind _tags (`Actor.Tags` OtherActor))
  (`|ExecutionSequence`
    (:`then_0`
      (if (and (`KismetArrayLibrary.Array_Contains` (`self.Tags`) "BulletEnemy") (`KismetArrayLibrary.Array_Contains` (`Actor.Tags` OtherActor) "Player"))
        (bind _asbp_character (cast `/Game/00_Space_Shooter/Player/BP_Character` (`GameplayStatics.GetPlayerPawn` 0)))
        (`/Game/00_Space_Shooter/Player/BP_Character.DamageActor` _asbp_character)
        (`GameplayStatics.SpawnEmitterAtLocation` "/Game/StarterContent/Particles/P_Explosion.P_Explosion" (`self.K2_GetActorLocation`) :!label _label)
        (`GameplayStatics.PlaySound2D` "/Game/StarterContent/Audio/Explosion02.Explosion02" 1.0 1.0 0.0 null null)
        (`KismetSystemLibrary.Delay` 0.2)
        (`self.K2_DestroyActor`)
        (else
          (if (or (`KismetArrayLibrary.Array_Contains` _tags "LimiteD") (`KismetArrayLibrary.Array_Contains` _tags "LimiteU")) :!label _label_2
            (`self.K2_DestroyActor`)))))
    (:`then_1`
      (if (and (`KismetArrayLibrary.Array_Contains` (`self.Tags`) "BulletPlayer") (`KismetArrayLibrary.Array_Contains` (`Actor.Tags` OtherActor) "Enemy"))
        (goto _label)
        (else
          (goto _label_2))))))

(fn `Move`
  (params (A :type "Float (single-precision)"))
  (`self.K2_SetActorLocation` (+ (`self.K2_GetActorLocation`) (* (`self.GetActorForwardVector`) (* A (`self.Speed`))))))

(fn `UserConstructionScript`)