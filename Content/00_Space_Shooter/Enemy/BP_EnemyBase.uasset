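; BP_EnemyBase is the base enemy actor for the space shooter, flying along its initial forward vector and firing bullets on a timer.
; Tick moves it without sweep and spawns a tagged bullet at FirePoint, aligned to the enemy's rotation, whenever the shoot delay elapses.
; Overlap with a BulletPlayer-tagged actor fires the destroy dispatcher, which destroys the enemy after a short delay, and reports BaseScore to BP_GameModeSpaceShooter.
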(event `self.ReceiveBeginPlay`
  (set `self.MovementVector` (`self.GetActorForwardVector`))
  (add `self.onEnemyDestroy` (delegate `Destroy_Event`)))

(event `Destroy_Event`
  (`KismetSystemLibrary.Delay` 0.2)
  (`self.K2_DestroyActor`))

(event `self.ReceiveActorBeginOverlap`
  (params (OtherActor :type "Actor Object Reference"))
  (if (`KismetArrayLibrary.Array_Contains` (`Actor.Tags` OtherActor) "BulletPlayer")
    (`self.onEnemyDestroy`)
    (bind _asbp_game_mode_space_shooter (cast `/Game/00_Space_Shooter/BP_GameModeSpaceShooter` (`GameplayStatics.GetGameMode`)))
    (`/Game/00_Space_Shooter/BP_GameModeSpaceShooter.EnemyDestroyed` _asbp_game_mode_space_shooter (`self.BaseScore`))))

(event `self.ReceiveTick`
  (params (DeltaSeconds :type "Float (single-precision)"))
  (`self.Move` DeltaSeconds)
  (bind _output_get (set `self.ShootCurrentTiem` (+ DeltaSeconds (`self.ShootCurrentTiem`))))
  (if (> _output_get (`self.DelayShoot`))
    (set `self.ShootCurrentTiem` 0.0)
    (`self.Fire`)))

(fn `Fire`
  (locals (Tags_bullet :type "Array of Name"))
  (bind _returnvalue (`|SpawnActorFromClass` (`self.Bullet`) (`SceneComponent.K2_GetComponentToWorld` (`self.FirePoint`)) "Undefined" "MultiplyWithRoot" null null))
  (`self.K2_SetActorRotation` _returnvalue (`self.K2_GetActorRotation`) false)
  (set `Actor.Tags` (`local.Tags_bullet`) _returnvalue))

(fn `Move`
  (params (DeltaTime :type "Float (double-precision)"))
  (`self.K2_SetActorLocation` (+ (`self.K2_GetActorLocation`) (* (`self.MovementVector`) (* DeltaTime (`self.Speed`))))))

(fn `UserConstructionScript`)