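; Horizontal enemy variant for the space shooter that moves sideways with a constant X offset, starting right or left at random.
; It sets the MovementVector on BeginPlay and leaves Tick disabled, adding behavior on top of its parent class.
; Overlapping an actor tagged "Lateral" toggles IsRight, shortening DelayShoot only when switching from right to left.
; Both toggle branches assign the same negated right vector, so the switch to right still points left.
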(event `self.ReceiveBeginPlay`
  (bind _returnvalue (`self.GetActorRightVector`))
  (`parent.ReceiveBeginPlay`)
  (if (`KismetMathLibrary.RandomBool`)
    (set `self.bIsRight` true)
    (set `self.MovementVector` (+ _returnvalue (0.5 0.0 0.0)))
    (else
      (set `self.bIsRight` false)
      (set `self.MovementVector` (+ (* _returnvalue -1.0) (0.5 0.0 0.0))))))

(event `self.ReceiveActorBeginOverlap`
  (params (OtherActor :type "Actor Object Reference"))
  (bind _returnvalue (* (`self.GetActorRightVector`) -1.0))
  (`parent.ReceiveActorBeginOverlap` OtherActor)
  (if (`KismetArrayLibrary.Array_Contains` (`Actor.Tags` OtherActor) "Lateral")
    (if (`self.bIsRight`)
      (set `self.bIsRight` false)
      (set `self.MovementVector` (+ _returnvalue (0.5 0.0 0.0)))
      (set `self.DelayShoot` (- (`self.DelayShoot`) 0.1))
      (else
        (set `self.bIsRight` true)
        (set `self.MovementVector` (+ _returnvalue (0.5 0.0 0.0)))))))

(fn `UserConstructionScript`
  (`parent.UserConstructionScript`))