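; Enemy spawner for the space shooter that spawns an enemy on a looping timer started at BeginPlay.
; Each spawn picks a random SpawnPoint-tagged component and an enemy class, base or horizontal, randomized by the game mode's Level and clamped.
; Spawn tries to bind each enemy's destroy event to lower SpawnTime, though the running timer is never reset to use it.
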(event `self.ReceiveBeginPlay`
  (`KismetSystemLibrary.K2_SetTimerDelegate` (delegate `Spawn`) (`self.SpawnTime`) true)
  (bind _asbp_game_mode_space_shooter (cast `/Game/00_Space_Shooter/BP_GameModeSpaceShooter` (`GameplayStatics.GetGameMode`)))
  (set `self.BPGameMode` _asbp_game_mode_space_shooter))

(event `Spawn`
  (bind _new_enemy (`self.SpawnEnemy`))
  (bind _asbp_enemy_base (cast `/Game/00_Space_Shooter/Enemy/BP_EnemyBase` _new_enemy))
  (add `/Game/00_Space_Shooter/Enemy/BP_EnemyBase.onEnemyDestroy` _asbp_enemy_base (delegate `Enemy_Destroyed`)))

(event `Enemy_Destroyed`
  (set `self.SpawnTime` (- (`self.SpawnTime`) 1.0)))

(fn `GetClassToSpawn`
  (params (Type :type Integer))
  (returns (NewClass :type "Actor Class Reference"))
  (return (select `int` (`KismetMathLibrary.Clamp` Type 0 (- (`self.MaxNumEnemies`) 1)) :`0` "/Game/00_Space_Shooter/Enemy/BP_EnemyBase.BP_EnemyBase_C" :`1` "/Game/00_Space_Shooter/Enemy/BP_Enemy_Horizontal.BP_Enemy_Horizontal_C" :!type "Actor Class Reference")))

(fn `SpawnEnemy`
  (returns (`New Enemy` :type "Actor Object Reference"))
  (bind _returnvalue (`self.GetComponentsByTag` "/Script/Engine.SceneComponent" "SpawnPoint"))
  (bind _newclass (`self.GetClassToSpawn` (`KismetMathLibrary.RandomInteger` (`/Game/00_Space_Shooter/BP_GameModeSpaceShooter.Level` (`self.BPGameMode`)))))
  (bind _returnvalue_2 (`|SpawnActorFromClass` _newclass (`SceneComponent.K2_GetComponentToWorld` (`|GetArrayItem` _returnvalue (`KismetMathLibrary.RandomInteger` (`KismetArrayLibrary.Array_Length` _returnvalue)))) "Undefined" "MultiplyWithRoot" null null))
  (bind _asbp_enemy_base (cast `/Game/00_Space_Shooter/Enemy/BP_EnemyBase` _returnvalue_2)
    (:`CastFailed`
      (return _asbp_enemy_base))))

(fn `UserConstructionScript`)