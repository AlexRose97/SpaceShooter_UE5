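; Game mode for the space shooter that tracks the run's distance, score and player death state.
; Tick adds a fixed increment to Distance until the player is dead.
; PlayerDeath casts player 0's HUD to BP_Hud, calls PlayerKill on it and sets the death flag, which halts distance tracking.
; EnemyDestroyed takes a score value and increases the Score total.
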(event `self.ReceiveTick`
  (params (DeltaSeconds :type "Float (single-precision)"))
  (if (not (`self.bIsDeath`))
    (set `self.Distance` (+ (`self.IncrementPerTick`) (`self.Distance`)))))

(event `PlayerDeath`
  (bind _asbp_hud (cast `/Game/00_Space_Shooter/UI/BP_Hud` (`PlayerController.GetHUD` (`GameplayStatics.GetPlayerController` 0))))
  (`/Game/00_Space_Shooter/UI/BP_Hud.PlayerKill` _asbp_hud)
  (set `self.bIsDeath` true))

(event `EnemyDestroyed`
  (params (Score :type Integer))
  (set `self.Score` (+ Score (`self.Score`))))

(fn `UserConstructionScript`)